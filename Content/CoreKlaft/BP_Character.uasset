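; Player pawn for the Klaft turn-based board game, shown as Veto, Mage, Barde or a default body by toggling capsule visibility.
; Initializes turn stats with random bonus action points (PA); each move spends one and ends the turn at zero.
; S_/M_ event pairs relay setup, montages and moves, which use rotate-then-translate timelines and update tile occupancy.
; Spawns its own following BP_Camera; destruction removes it and requests a controller respawn.
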(event `C_SetupCharacterPlayer`
  (params (Selection :type Name) (RefInfoPlayer :type "/Game/CoreKlaft/ST_CaracPlayer2 Structure"))
  (`self.M_SetupCharacterPlayer` Selection))

(event `S_SetupCharacterPlayer`
  (params (Selection :type Name) (RefInfoPlayer :type "/Game/CoreKlaft/ST_CaracPlayer2 Structure"))
  (`self.M_SetupCharacterPlayer` Selection RefInfoPlayer))

(event `M_SetupCharacterPlayer`
  (params (Selection :type Name) (RefInfoPlayer :type "/Game/CoreKlaft/ST_CaracPlayer2 Structure"))
  (set `self.RefInfoPlayer` RefInfoPlayer)
  (switch `name` Selection
    (:`Veto`
      (`SceneComponent.SetVisibility` (`self.CapsuleVeto`) true true)
      (`SceneComponent.SetVisibility` (`self.CapsuleMage`) false true)
      (`SceneComponent.SetVisibility` (`self.CapsuleBarde`) false true)
      (`SceneComponent.SetVisibility` (`self.CapsuleCharacterDefault`) false true)
      (cast `/Game/CoreKlaft/PC_KlaftGame` (`self.GetController`) :!label _label))
    (:`Mage`
      (`SceneComponent.SetVisibility` (`self.CapsuleMage`) true true)
      (`SceneComponent.SetVisibility` (`self.CapsuleVeto`) false true)
      (`SceneComponent.SetVisibility` (`self.CapsuleBarde`) false true)
      (`SceneComponent.SetVisibility` (`self.CapsuleCharacterDefault`) false true)
      (goto _label))
    (:`Barde`
      (`SceneComponent.SetVisibility` (`self.CapsuleBarde`) true true)
      (`SceneComponent.SetVisibility` (`self.CapsuleVeto`) false true)
      (`SceneComponent.SetVisibility` (`self.CapsuleMage`) false true)
      (`SceneComponent.SetVisibility` (`self.CapsuleCharacterDefault`) false true)
      (goto _label))
    (:`None`
      (`SceneComponent.SetVisibility` (`self.CapsuleCharacterDefault`) true true)
      (`SceneComponent.SetVisibility` (`self.CapsuleVeto`) false true)
      (`SceneComponent.SetVisibility` (`self.CapsuleMage`) false true)
      (`SceneComponent.SetVisibility` (`self.CapsuleBarde`) false true))))

(event `self.ReceiveBeginPlay`
  (`|ExecutionSequence`
    (:`then_0`
      (set `self.RandomPaValue` (`KismetMathLibrary.RandomIntegerInRange` 1 5))
      (`self.S_IniatilisationTour`)
      (`/Game/CoreKlaft/PC_KlaftGame.M_SetAxisBoard` (cast `/Game/CoreKlaft/PC_KlaftGame` (`self.GetController`) :!pure true) false)
      (`KismetSystemLibrary.Delay` 5.0)
      (`self.CreateCameraPlayer`))))

(event `S_IniatilisationTour`
  (bind (_refinfoplayer_posture _refinfoplayer_attaque _refinfoplayer_defense _refinfoplayer_vitesse _refinfoplayer_pa) (break `/Game/CoreKlaft/ST_CaracPlayer2` (`self.RefInfoPlayer`)))
  (set `self.PlayerInfoCurrentGame` (make `/Game/CoreKlaft/ST_CaracPlayer2` _refinfoplayer_posture _refinfoplayer_attaque _refinfoplayer_defense _refinfoplayer_vitesse (+ _refinfoplayer_pa (`self.RandomPaValue`)))))

(event `S_Moving`
  (params (NewParam :type "Vector Structure"))
  (bind (_playerinfocurrentgame_posture _playerinfocurrentgame_attaque _playerinfocurrentgame_defense _playerinfocurrentgame_vitesse _playerinfocurrentgame_pa) (break `/Game/CoreKlaft/ST_CaracPlayer2` (`self.PlayerInfoCurrentGame`)))
  (bind (_playerinfocurrentgame_posture_2 _playerinfocurrentgame_attaque_2 _playerinfocurrentgame_defense_2 _playerinfocurrentgame_vitesse_2 _playerinfocurrentgame_pa_2) (break `/Game/CoreKlaft/ST_CaracPlayer2` (`self.PlayerInfoCurrentGame`)))
  (bind _returnvalue (- _playerinfocurrentgame_pa 1))
  ;[0 0.8887 1] Pa Module
  (if (> _playerinfocurrentgame_pa_2 0)
    (if (== _returnvalue 0)
      (set `self.IsMyTour?` false))
    (set `self.PlayerInfoCurrentGame` (make `/Game/CoreKlaft/ST_CaracPlayer2` _playerinfocurrentgame_posture _playerinfocurrentgame_attaque _playerinfocurrentgame_defense _playerinfocurrentgame_vitesse _returnvalue))
    (`self.S_MovingInializationAction` NewParam)
    (else
      (set `self.IsMyTour?` false))))

(event `CreateCameraPlayer`
  (bind _socketcamera2 (`self.SocketCamera2`))
  (bind (_returnvalue_location _returnvalue_rotation) (`KismetMathLibrary.BreakTransform` (`SceneComponent.K2_GetComponentToWorld` _socketcamera2)))
  ;[1 1 1] Comment
  (bind _returnvalue (`|SpawnActorFromClass` "/Game/CoreKlaft/BP_Camera.BP_Camera_C" (`KismetMathLibrary.MakeTransform` _returnvalue_location (`KismetMathLibrary.MakeRotator` 0.0 0.0 (.yaw _returnvalue_rotation))) "Undefined" "OverrideRootScale" null self (`SceneComponent.RelativeLocation` _socketcamera2) (`SceneComponent.RelativeLocation` (`self.SocketCamera1`)) null))
  (bind _output_get (set `self.RefCamera` _returnvalue))
  (`SceneComponent.K2_SetWorldRotation` (`/Game/CoreKlaft/BP_Camera.Camera` _output_get) _returnvalue_rotation false false)
  (`PlayerController.SetViewTargetWithBlend` (cast `/Game/CoreKlaft/PC_KlaftGame` (`self.GetController` self) :!pure true) _output_get 0.0 "VTBlend_Linear" 0.0 false))

(event `M_ChangeStateAnim`
  (params (SateANim :type "/Game/CoreKlaft/EListStateAnim Enum" :default "NewEnumerator0") (Selection :type Name))
  (switch `name` Selection
    (:`Veto`
      (`|PlayMontage` (`self.SkeletalMeshVeto`) (select `/Game/CoreKlaft/EListStateAnim` SateANim :`NewEnumerator3` "/Game/LucasNayrac/Animation/Veto/Anim_Veto_EngagementCombat_Victoire_Montage.Anim_Veto_EngagementCombat_Victoire_Montage" :`NewEnumerator2` "/Game/LucasNayrac/Animation/Veto/Anim_Veto_Mort_Montage.Anim_Veto_Mort_Montage" :`NewEnumerator4` "/Game/LucasNayrac/Animation/Veto/Anim_Veto_PerdreCorruption_Montage.Anim_Veto_PerdreCorruption_Montage" :`NewEnumerator5` "/Game/LucasNayrac/Animation/Veto/Anim_Veto_AspirerCorruption_Montage.Anim_Veto_AspirerCorruption_Montage" :`NewEnumerator6` "/Game/LucasNayrac/Animation/Veto/Anim_Veto_Defaite_Montage.Anim_Veto_Defaite_Montage" :`NewEnumerator7` "/Game/LucasNayrac/Animation/Veto/Anim_Veto_Victoire_Montage.Anim_Veto_Victoire_Montage" :`NewEnumerator8` "/Game/LucasNayrac/Animation/Veto/Anim_Veto_Agonie_Montage.Anim_Veto_Agonie_Montage" :`NewEnumerator9` "/Game/LucasNayrac/Animation/Veto/Anim_Veto_PrendreCoup_Montage.Anim_Veto_PrendreCoup_Montage" :`NewEnumerator10` "/Game/LucasNayrac/Animation/Veto/Anim_Veto_DonnerCoup_Montage.Anim_Veto_DonnerCoup_Montage" :!type "AnimMontage Object Reference")))
    (:`Mage`
      (`|PlayMontage` (`self.SkeletalMeshMage`) (select `/Game/CoreKlaft/EListStateAnim` SateANim :`NewEnumerator3` "/Game/LucasNayrac/Animation/Mage/Anim_Mage_EngagementCombat_Victoire_Montage.Anim_Mage_EngagementCombat_Victoire_Montage" :`NewEnumerator2` "/Game/LucasNayrac/Animation/Mage/Anim_Mage_Mort_Montage.Anim_Mage_Mort_Montage" :`NewEnumerator4` "/Game/LucasNayrac/Animation/Mage/Anim_Mage_PerdreCorruption_Montage.Anim_Mage_PerdreCorruption_Montage" :`NewEnumerator5` "/Game/LucasNayrac/Animation/Mage/Anim_Mage_AspirerCorruption_Montage.Anim_Mage_AspirerCorruption_Montage" :`NewEnumerator6` "/Game/LucasNayrac/Animation/Mage/Anim_Mage_Defaite_Montage.Anim_Mage_Defaite_Montage" :`NewEnumerator7` "/Game/LucasNayrac/Animation/Mage/Anim_Mage_Victoire_Montage.Anim_Mage_Victoire_Montage" :`NewEnumerator8` "/Game/LucasNayrac/Animation/Mage/Anim_Mage_Agonie_Montage.Anim_Mage_Agonie_Montage" :`NewEnumerator9` "/Game/LucasNayrac/Animation/Mage/Anim_Mage_PrendreCoup_Montage.Anim_Mage_PrendreCoup_Montage" :`NewEnumerator10` "/Game/LucasNayrac/Animation/Mage/Anim_Mage_DonnerCoup_Montage.Anim_Mage_DonnerCoup_Montage" :!type "AnimMontage Object Reference")))
    (:`Barde`
      (`|PlayMontage` (`self.SkeletalMeshBarde`) (select `/Game/CoreKlaft/EListStateAnim` SateANim :`NewEnumerator3` "/Game/LucasNayrac/Animation/Barde/Anim_Barde_EngagementCombat_Victoire_BrandirArme_Montage.Anim_Barde_EngagementCombat_Victoire_BrandirArme_Montage" :`NewEnumerator2` "/Game/LucasNayrac/Animation/Barde/Anim_Barde_Mort_Montage.Anim_Barde_Mort_Montage" :`NewEnumerator4` "/Game/LucasNayrac/Animation/Barde/Anim_Barde_PerdreCorruption_Montage.Anim_Barde_PerdreCorruption_Montage" :`NewEnumerator5` "/Game/LucasNayrac/Animation/Barde/Anim_Barde_AspirerCorruption_Montage.Anim_Barde_AspirerCorruption_Montage" :`NewEnumerator6` "/Game/LucasNayrac/Animation/Barde/Anim_Barde_Defaite_Montage.Anim_Barde_Defaite_Montage" :`NewEnumerator7` "/Game/LucasNayrac/Animation/Barde/Anim_Barde_Victoire_Montage.Anim_Barde_Victoire_Montage" :`NewEnumerator8` "/Game/LucasNayrac/Animation/Barde/Anim_Barde_Agonie_Montage.Anim_Barde_Agonie_Montage" :`NewEnumerator9` "/Game/LucasNayrac/Animation/Barde/Anim_Barde_PrendreCoup_Montage.Anim_Barde_PrendreCoup_Montage" :`NewEnumerator10` "/Game/LucasNayrac/Animation/Barde/Anim_Barde_DonnerCoup_Montage.Anim_Barde_DonnerCoup_Montage" :!type "AnimMontage Object Reference")))))

(event `S_ChangeAnimState`
  (params (SateANim :type "/Game/CoreKlaft/EListStateAnim Enum" :default "NewEnumerator0") (NameCharacter :type Name))
  (`self.M_ChangeStateAnim` SateANim NameCharacter))

(event `S_MovingInializationAction`
  (params (NewParam :type "Vector Structure") (`RefTile?` :type "/Game/Klaft/Blueprint/BP_TileContenerGrid Object Reference"))
  (`self.M_MovingPawn` NewParam `RefTile?`))

(event `M_MovingPawn`
  (params (LoctionPlayerTarget :type "Vector Structure") (`RefTile?` :type "/Game/Klaft/Blueprint/BP_TileContenerGrid Object Reference"))
  (if (not (`self.PawnMoving?`))
    (set `self.PawnMoving?` true)
    (set `self.LoctionPlayerTarget` LoctionPlayerTarget)
    (set `self.LocationPlayerStart` (`self.K2_GetActorLocation`))
    (set `self.RotationCameraStart` (`self.K2_GetActorRotation`))
    (`/Game/CoreKlaft/BP_Camera.SetupPointForReset` (`self.RefCamera`) self)
    (set `self.SateANim` "NewEnumerator1")
    (set `/Game/Klaft/Blueprint/BP_TileContenerGrid.PlayerIsHere?` false (`self.RefTile?`))
    (`self.S_SetPlayerIsHereTile` false)
    (set `self.RefTile?` `RefTile?`)
    ;[1 1 1] Step 1 : Rotation Pawn
    (bind (_direction _percentanim) (`Timeline|AnimRotate` :!via `PlayFromStart`)
      (:`Update`
        (`self.SetrotationPawn` _percentanim))
      (:`Finished`
        ;[1 1 1] Step 2 : Move pawn
        (bind (_direction_2 _percentanim_2) (`Timeline|AnimMove` :!via `PlayFromStart`)
          (:`Update`
            (`self.SetLocationPawn` _percentanim_2)
            (`/Game/CoreKlaft/BP_Camera.FixCameraLocation` (`self.RefCamera`) self))
          (:`Finished`
            (set `self.PawnMoving?` false)
            (set `/Game/CoreKlaft/PC_KlaftGame.ActionLaunch` false (cast `/Game/CoreKlaft/PC_KlaftGame` (`self.GetController` self) :!pure true))
            (set `self.SateANim` "NewEnumerator0")
            (set `/Game/Klaft/Blueprint/BP_TileContenerGrid.PlayerIsHere?` true (`self.RefTile?`))
            (`self.S_SetPlayerIsHereTile` true self)))))))

(event `self.ReceiveDestroyed`
  (`self.K2_DestroyActor` (`self.RefCamera`))
  (bind _aspc_klaft_game (cast `/Game/CoreKlaft/PC_KlaftGame` (`self.GetController`)))
  (`/Game/CoreKlaft/PC_KlaftGame.S_RespawnPlayer` _aspc_klaft_game))

(event `S_SetPlayerIsHereTile`
  (params (`PlayerIsHere?` :type Boolean) (RefPlayerIsHere :type "Pawn Object Reference"))
  (bind _reftile_ (`self.RefTile?`))
  (set `/Game/Klaft/Blueprint/BP_TileContenerGrid.PlayerIsHere?` `PlayerIsHere?` _reftile_)
  (set `/Game/Klaft/Blueprint/BP_TileContenerGrid.RefPlayerIsHere` RefPlayerIsHere _reftile_))

(fn `GetAxisForwardCharcter`
  (returns (`Axis X ?` :type Boolean))
  (bind (_returnvalue_x _returnvalue_y) (`KismetMathLibrary.BreakVector` (`self.GetActorForwardVector`)))
  (if (> _returnvalue_x 0.0)
    (return true)
    (elif (> _returnvalue_y 0.0)
      (return false))))

(fn `NewFunction_0`
  (params (Selection :type Name))
  (switch `name` Selection))

(fn `OnRep_InfoPlayer`)

(fn `OnRep_IsMyTour?`)

(fn `OnRep_NewVar_0`)

(fn `OnRep_PlayerInfoCurrentGame`)

(fn `OnRep_SateANim`)

(fn `SetLocationPawn`
  (params (Alpha :type "Float (double-precision)"))
  (returns (LerpValue :type "Vector Structure"))
  (bind _returnvalue (`KismetMathLibrary.VLerp` (`self.LocationPlayerStart`) (`KismetMathLibrary.MakeVector` (.x (`self.LoctionPlayerTarget`)) (.y (`self.LoctionPlayerTarget`)) (.z (`self.LocationPlayerStart`))) Alpha))
  (`self.K2_SetActorLocation` _returnvalue)
  (return _returnvalue))

(fn `SetrotationPawn`
  (params (Alpha :type "Float (double-precision)"))
  (bind (_rotationcamerastart_roll _rotationcamerastart_pitch) (`KismetMathLibrary.BreakRotator` (`self.RotationCameraStart`)))
  (bind (_returnvalue_roll _returnvalue_pitch _returnvalue_yaw) (`KismetMathLibrary.BreakRotator` (`KismetMathLibrary.FindLookAtRotation` (`self.LocationPlayerStart`) (`self.LoctionPlayerTarget`))))
  (`self.K2_SetActorRotation` (`KismetMathLibrary.RLerp` (`self.RotationCameraStart`) (`KismetMathLibrary.MakeRotator` _rotationcamerastart_roll _rotationcamerastart_pitch _returnvalue_yaw) Alpha true)))

(fn `SetupTimeAnim`
  (`TimelineComponent.SetPlayRate` (`self.AnimRotate`) (/ 1.0 (`self.DurationAnimRotate`)))
  (`TimelineComponent.SetPlayRate` (`self.AnimMove`) (/ 1.0 (`self.DurationAnimMove`))))

(fn `UserConstructionScript`)