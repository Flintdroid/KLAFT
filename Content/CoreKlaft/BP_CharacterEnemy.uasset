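; Enemy character for the Klaft game that plays combat montages and turns to face a target location.
; S_ChangeAnimState selects a montage by enemy type (Bandit, Lezard, Pantin) and state index, with many states still unassigned.
; S_RotateEnemy forwards to M_RotateEnemy, where a timeline lerps yaw toward the target while StateAnim switches from Run to Idle.
; The OnRep handlers are empty, and the position-lerp helper is not called here.
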(event `S_ChangeAnimState`
  (params (Index :type "/Game/CoreKlaft/EListStateAnim Enum" :default "NewEnumerator0"))
  (switch `name` (`self.NameEnemy`)
    (:`Bandit`
      (`|PlayMontage` (`self.SkeletalMesh`) (select `/Game/CoreKlaft/EListStateAnim` Index :`NewEnumerator3` "/Game/LucasNayrac/Animation/Bandit/Anim_Bandit_EngagementCombat_Victoire_Montage.Anim_Bandit_EngagementCombat_Victoire_Montage" :`NewEnumerator10` "/Game/LucasNayrac/Animation/Bandit/Anim_Bandit_DonnerCoup_Montage.Anim_Bandit_DonnerCoup_Montage" :!type "AnimMontage Object Reference")))
    (:`Lezard`
      (`|PlayMontage` (`self.SkeletalMesh`) (select `/Game/CoreKlaft/EListStateAnim` Index :`NewEnumerator0` "/Game/LucasNayrac/Animation/Lezard/Anim_Lizou_Idle_Montage.Anim_Lizou_Idle_Montage" :`NewEnumerator3` "/Game/LucasNayrac/Animation/Lezard/Anim_Lizou_EngagementCombat_Montage.Anim_Lizou_EngagementCombat_Montage" :`NewEnumerator2` "/Game/LucasNayrac/Animation/Lezard/Anim_Lizou_Mort_Montage.Anim_Lizou_Mort_Montage" :`NewEnumerator10` "/Game/LucasNayrac/Animation/Lezard/Anim_Lizou_DonnerCoup_Montage.Anim_Lizou_DonnerCoup_Montage" :!type "AnimMontage Object Reference")))
    (:`Pantin`
      (`|PlayMontage` (`self.SkeletalMesh`) (select `/Game/CoreKlaft/EListStateAnim` Index :`NewEnumerator0` "/Game/LucasNayrac/Animation/Pantin/Anim_Pantin_Idle_Montage.Anim_Pantin_Idle_Montage" :`NewEnumerator3` "/Game/LucasNayrac/Animation/Pantin/Anim_Pantin_EngagementCombat_Victoire_Montage.Anim_Pantin_EngagementCombat_Victoire_Montage" :`NewEnumerator2` "/Game/LucasNayrac/Animation/Pantin/Anim_Pantin_Mort_Montage.Anim_Pantin_Mort_Montage" :`NewEnumerator9` "/Game/LucasNayrac/Animation/Pantin/Anim_Pantin_PrendreCoup_Montage.Anim_Pantin_PrendreCoup_Montage" :`NewEnumerator10` "/Game/LucasNayrac/Animation/Pantin/Anim_Pantin_DonnerCoup_Montage.Anim_Pantin_DonnerCoup_Montage" :!type "AnimMontage Object Reference")))))

(event `S_RotateEnemy`
  (params (LocationTarget :type "Vector Structure"))
  (`self.M_RotateEnemy` LocationTarget))

(event `M_RotateEnemy`
  (params (LoctionTarget :type "Vector Structure"))
  (if (not (`self.PawnMoving?`))
    (set `self.PawnMoving?` true)
    (set `self.LoctionPlayerTarget` LoctionTarget)
    (set `self.LocationPlayerStart` (`self.K2_GetActorLocation`))
    (set `self.RotationCameraStart` (`self.K2_GetActorRotation`))
    (set `self.StateAnim` "NewEnumerator1")
    ;[1 1 1] Step 1 : Rotation Pawn
    (bind (_direction _percentanim) (`Timeline|AnimRotate` :!via `PlayFromStart`)
      (:`Update`
        (`self.SetrotationPawn` _percentanim))
      (:`Finished`
        (set `self.StateAnim` "NewEnumerator0")))))

(fn `OnRep_InfoPlayer`)

(fn `OnRep_IsMyTour?`)

(fn `OnRep_NewVar_0`)

(fn `OnRep_PlayerInfoCurrentGame`)

(fn `OnRep_StateAnim`)

(fn `SetLocationPawn`
  (params (Alpha :type "Float (double-precision)"))
  (`self.K2_SetActorLocation` (`KismetMathLibrary.VLerp` (`self.LocationPlayerStart`) (`KismetMathLibrary.MakeVector` (.x (`self.LoctionPlayerTarget`)) (.y (`self.LoctionPlayerTarget`)) (.z (`self.LocationPlayerStart`))) Alpha)))

(fn `SetrotationPawn`
  (params (Alpha :type "Float (double-precision)"))
  (bind (_rotationcamerastart_roll _rotationcamerastart_pitch) (`KismetMathLibrary.BreakRotator` (`self.RotationCameraStart`)))
  (bind (_returnvalue_roll _returnvalue_pitch _returnvalue_yaw) (`KismetMathLibrary.BreakRotator` (`KismetMathLibrary.FindLookAtRotation` (`self.LocationPlayerStart`) (`self.LoctionPlayerTarget`))))
  (`self.K2_SetActorRotation` (`KismetMathLibrary.RLerp` (`self.RotationCameraStart`) (`KismetMathLibrary.MakeRotator` _rotationcamerastart_roll _rotationcamerastart_pitch _returnvalue_yaw) Alpha true)))

(fn `SetupTimeAnim`
  (`TimelineComponent.SetPlayRate` (`self.AnimRotate`) (/ 1.0 (`self.DurationAnimRotate`))))

(fn `UserConstructionScript`)