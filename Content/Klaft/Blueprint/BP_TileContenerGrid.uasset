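; Replicated board-grid tile that holds a two-sided flippable tile, its type, enemy, light and shop lists.
; Construction attaches two BP_Tileversoin2 child actors back to back on a pivot and derives movement, flip and enemy flags from type, randomizing Forest backs.
; A timeline rotates the pivot 180°, then can spawn a random region-based enemy and start the player's fight.
; S_/M_ event pairs relay changes, while RepNotifies toggle move and monster icons.
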(event `S_SetupTile2ForForest`
  (set `self.TypeTile_2` (select `int` (`KismetMathLibrary.RandomIntegerInRange` 0 2) :`0` "NewEnumerator9" :`1` "NewEnumerator10" :`2` "NewEnumerator5" :!type "/Game/Klaft/EListTypeTile Enum")))

(event `self.ReceiveBeginPlay`
  (`TimelineComponent.SetPlayRate` (`self.Animation`) (/ 1.0 (`self.DurationAnimation`)))
  (`/Engine/EditorBlueprintResources/ActorMacros.Switch Has Authority`
    (:`Authority`
      (`self.S_ConstructionScript`)
      (`self.S_TileAnimationConfiguration`)
      (`|ExecutionSequence`
        (:`then_0`
          (if (`|EnumEquality` (`self.TypeTile`) "NewEnumerator0")
            (`self.S_SetupTile2ForForest`)))
        (:`then_1`
          (if (`|EnumEquality` (`self.GetInfoTileIndex` 0) "NewEnumerator4")
            (set `self.RespawnPossible` true)))
        (:`then_2`
          (if (`|EnumEquality` (`self.TypeTile`) "NewEnumerator1")
            (`self.S_SpawnEnemy` null)))))))

(event `S_RemoveLight`
  (`self.K2_DestroyActor` (`self.RefLighting`)))

(event `S_SpawnLight`
  (params (TypeTyle :type "/Game/Klaft/EListTypeTile Enum" :default "NewEnumerator0"))
  (`self.M_SpawnLight` TypeTyle))

(event `M_SpawnLight`
  (params (Index :type "/Game/Klaft/EListTypeTile Enum" :default "NewEnumerator0"))
  (bind _returnvalue (`|SpawnActorFromClass` (select `/Game/Klaft/EListTypeTile` Index :`NewEnumerator0` "/Game/Kyllian/Valid/Assets/Lights/BP_Lights_CaseForet.BP_Lights_CaseForet_C" :`NewEnumerator1` "/Game/Kyllian/Valid/Assets/Lights/BP_Lights_CaseMonstre.BP_Lights_CaseMonstre_C" :`NewEnumerator2` "/Game/Kyllian/Valid/Assets/Lights/BP_Lights_CasePlaine.BP_Lights_CasePlaine_C" :`NewEnumerator3` "/Game/Kyllian/Valid/Assets/Lights/BP_Lights_CaseMontagne.BP_Lights_CaseMontagne_C" :`NewEnumerator4` "/Game/Kyllian/Valid/Assets/Lights/BP_Lights_CaseCristallerie.BP_Lights_CaseCristallerie_C" :`NewEnumerator5` "/Game/Kyllian/Valid/Assets/Lights/BP_Lights_CaseRoulotte.BP_Lights_CaseRoulotte_C" :`NewEnumerator6` "/Game/Kyllian/Valid/Assets/Lights/BP_Lights_CasePlaine.BP_Lights_CasePlaine_C" :`NewEnumerator7` "/Game/Kyllian/Valid/Assets/Lights/BP_Lights_CaseSyncristal_Gauche.BP_Lights_CaseSyncristal_Gauche_C" :`NewEnumerator8` "/Game/Kyllian/Valid/Assets/Lights/BP_Lights_CaseSyncristal.BP_Lights_CaseSyncristal_C" :`NewEnumerator9` "/Game/Kyllian/Valid/Assets/Lights/BP_Lights_CaseForet.BP_Lights_CaseForet_C" :`NewEnumerator10` "/Game/Kyllian/Valid/Assets/Lights/BP_Lights_CaseForet.BP_Lights_CaseForet_C" :!type "Actor Class Reference") (`KismetMathLibrary.MakeTransform` (`self.K2_GetActorLocation` self)) "Undefined" "OverrideRootScale" null null))
  (set `self.RefLighting` _returnvalue))

(event `S_TileAnimationConfiguration`
  (if (`|EnumEquality` (`self.GetInfoTileIndex` 0) "NewEnumerator2")
    (set `self.AnimationPossible` false)))

(event `S_SetCardList`
  (params (LIstCardInShop :type "Array of /Game/Florian/Interface/Tool/ST_CardsInfos Structure (by ref)"))
  (`self.M_SetCardList` LIstCardInShop))

(event `M_TileAnimationConfiguration`)

(event `M_SetCardList`
  (params (LIstCardInShop :type "Array of /Game/Florian/Interface/Tool/ST_CardsInfos Structure"))
  (set `self.LIstCardInShop` LIstCardInShop))

(event `S_SetGemmeList`
  (params (ListGemmeInShop :type "Array of /Game/CoreKlaft/ST_CaracPlayer2 Structure"))
  (`self.M_SetGemmeList` ListGemmeInShop))

(event `M_SetGemmeList`
  (params (ListGemmeInShop :type "Array of /Game/CoreKlaft/ST_CaracPlayer2 Structure"))
  (set `self.ListGemmeInShop` ListGemmeInShop))

(event `M_Construction`
  (if (`self.TransitionTile?`)
    (set `self.IndexTransition` (+ (`self.RegionIndex`) 1)))
  (`self.ConstructionStr`))

(event `S_ConstructionScript`
  (`self.M_Construction`))

(event `S_InitializeAnimTile`
  (params (PC :type "/Game/CoreKlaft/PC_KlaftGame Object Reference"))
  (bind _relative_rotation (`self.Relative Rotation`))
  (bind _pivottile (`self.PivotTile`))
  (bind _returnvalue (+ (`self.IndexTileType?`) 1))
  (if (`self.AnimationPossible`)
    (if (not (`self.AnimationIsPlaying?`))
      (set `self.AnimationIsPlaying?` true)
      (set `self.Relative Rotation` (`SceneComponent.K2_GetComponentRotation` _pivottile))
      (bind _isa (`/Engine/EditorBlueprintResources/StandardMacros.FlipFlop`)
        (:`A`
          _)
        (:`B`
          _))
      (`self.OptimizationViewPortTile` _isa)
      (bind (_direction _percentanimation) (`Timeline|Animation` :!via `PlayFromStart`)
        (:`Update`
          (`SceneComponent.K2_SetWorldRotation` _pivottile (`KismetMathLibrary.RLerp` _relative_rotation (`KismetMathLibrary.ComposeRotators` _relative_rotation (struct :`Pitch` 180.0)) _percentanimation true) false false))
        (:`Finished`
          (set `self.IndexTileType?` (select `bool` (> _returnvalue (`self.CountRotateTile`)) :`false` _returnvalue :`true` (`self.IndexTileType?`)))
          (set `self.Relative Rotation` (`self.K2_GetActorRotation`))
          (set `self.AnimationIsPlaying?` false)
          (if (`self.TournoiMode?`)
            (`/Game/CoreKlaft/PC_KlaftGame.S_SetTournoiMode` PC true))
          (if (`.Enemy_T1` (`self.GetInfoTileIndex` (`self.IndexTileType?`)))
            (`self.S_SpawnEnemy` PC)
            (`SceneComponent.K2_SetWorldRotation` (`self.IconPOssibleMove`) (struct :`Pitch` 180.0) true false)))))
    (elif (`.Enemy_T1` (`self.GetInfoTileIndex` (`self.IndexTileType?`)))
      (`self.S_SpawnEnemy` PC)
      (`SceneComponent.K2_SetWorldRotation` (`self.IconPOssibleMove`) (struct :`Pitch` 180.0) true false)
      (`KismetSystemLibrary.PrintString` "mdr!!!!!!!!!!"))))

(event `S_SpawnEnemy`
  (params (PC :type "/Game/CoreKlaft/PC_KlaftGame Object Reference"))
  (bind _returnvalue (`KismetMathLibrary.RandomIntegerInRange` 0 2))
  (`/Engine/EditorBlueprintResources/StandardMacros.IsValid` (`self.RefEnemyPawn`)
    (:`Is Valid`
      (`/Game/CoreKlaft/PC_KlaftGame.S_FightSystemModuleInitialization` PC (`self.RefEnemyPawn`) null null))
    (:`Is Not Valid`
      (`KismetSystemLibrary.PrintString` (`KismetStringLibrary.Conv_IntToString` (`self.IndexTileType?`)) true true (struct :`R` 1.0 :`G` 0.965232 :`A` 1.0) 50.0)
      (bind _returnvalue_2 (`|SpawnActorFromClass` (select `int` (`.RegionIndex` (`self.GetInfoTileIndex` (`self.IndexTileType?`))) :`0` (select `int` _returnvalue :`0` "/Game/Bandit01.Bandit01_C" :`1` "/Game/Lezard01.Lezard01_C" :`2` "/Game/Pantin01.Pantin01_C" :!type "Actor Class Reference") :`1` (select `int` _returnvalue :`0` "/Game/Bandit02.Bandit02_C" :`1` "/Game/Lezard02.Lezard02_C" :`2` "/Game/Pantin02.Pantin02_C" :!type "Actor Class Reference") :`2` (select `int` _returnvalue :`0` "/Game/Bandit03.Bandit03_C" :`1` "/Game/Lezard03.Lezard03_C" :`2` "/Game/Pantin03.Pantin03_C" :!type "Actor Class Reference")) (`KismetMathLibrary.Conv_VectorToTransform` (+ (`self.K2_GetActorLocation`) (0.0 0.0 96.0))) "Undefined" "OverrideRootScale" null null))
      (bind _asbp_character_enemy (cast `/Game/CoreKlaft/BP_CharacterEnemy` _returnvalue_2))
      (bind _output_get (set `self.RefEnemyPawn` _asbp_character_enemy))
      (`/Engine/EditorBlueprintResources/StandardMacros.IsValid` PC
        (:`Is Valid`
          (`/Game/CoreKlaft/BP_CharacterEnemy.S_RotateEnemy` _output_get (`self.K2_GetActorLocation` (`Controller.K2_GetPawn` PC)))
          (`/Game/CoreKlaft/PC_KlaftGame.S_FightSystemModuleInitialization` PC (`self.RefEnemyPawn`) null null))))))

(fn `GetInfoTileIndex`
  (params (Selection :type Integer))
  (returns (TypeTile :type "/Game/Klaft/EListTypeTile Enum") (Enemy_T1 :type Boolean) (ClassEnemy_T1 :type "/Game/CoreKlaft/BP_CharacterEnemy Class Reference") (RegionIndex :type Integer))
  (bind _regionindex (`self.RegionIndex`))
  (switch `int` Selection
    (:`0`
      (return "NewEnumerator0" false "/Game/Pantin03.Pantin03_C" _regionindex))
    (:`1`
      (return (`self.TypeTile`) (`self.Enemy_T1`) (`self.ClassEnemy_T1`) _regionindex))
    (:`2`
      (return (`self.TypeTile_2`) (`self.Enemy_T2`) (`self.ClassEnemy_T2`) _regionindex))
    (:`3`
      (return (`self.TypeTile_3`) (`self.Enemy_T3`) (`self.ClassEnemy_T3`) _regionindex))
    (:`4`
      (return (`self.TypeTile_4`) (`self.Enemy_T4`) (`self.ClassEnemy_T4`) _regionindex))
    (:`5`
      (return (`self.TypeTile_5`) (`self.Enemy_T5`) (`self.ClassEnemy_T5`) _regionindex))))

(fn `OnRep_AnimationPossible`)

(fn `OnRep_Enemy_T2`)

(fn `OnRep_EnemyIsHere?`
  (bind _iconmonster (`self.IconMonster`))
  (if (`self.EnemyIsHere?`)
    (`SceneComponent.SetVisibility` _iconmonster true true)
    (else
      (`SceneComponent.SetVisibility` _iconmonster false true))))

(fn `OnRep_IndexTileType?`)

(fn `OnRep_LIstCardInShop`)

(fn `OnRep_ListGemmeInShop`)

(fn `OnRep_NbItemCreate`)

(fn `OnRep_PlayerIsHere?`
  (bind _iconpossiblemove (`self.IconPOssibleMove`))
  (if (`self.PlayerIsHere?`)
    (`SceneComponent.SetVisibility` _iconpossiblemove true true)
    (else
      (`SceneComponent.SetVisibility` _iconpossiblemove false true))))

(fn `OnRep_POssibleToMove?`)

(fn `OnRep_RefEnemyPawn`
  (`/Engine/EditorBlueprintResources/StandardMacros.IsValid` (`self.RefEnemyPawn`)
    (:`Is Valid`
      (set `self.EnemyIsHere?` true))
    (:`Is Not Valid`
      (set `self.EnemyIsHere?` false))))

(fn `OnRep_RefLighting`)

(fn `OnRep_RefPlayerIsHere`
  (if (not (`self.PlayerIsHere?`))
    (set `self.RefPlayerIsHere` null)))

(fn `OnRep_RespawnPossible`)

(fn `OnRep_TournoiMode?`)

(fn `OnRep_TransitionTile?`)

(fn `OnRep_TypeTile`)

(fn `OnRep_TypeTile_2`)

(fn `OnRep_TypeTile_3`)

(fn `OptimizationViewPortTile`
  (params (`Is A` :type Boolean))
  (`SceneComponent.SetVisibility` (select `bool` `Is A` :`false` (`self.Tile1`) :`true` (`self.Tile2`) :!type "SceneComponent Object Reference") true true)
  (`SceneComponent.SetVisibility` (select `bool` `Is A` :`false` (`self.Tile2`) :`true` (`self.Tile1`) :!type "SceneComponent Object Reference") false true))

(fn `setupConstruction`
  (`/Game/Klaft/Blueprint/BP_Tileversoin2.SetupTile` (cast `/Game/Klaft/Blueprint/BP_Tileversoin2` (`ChildActorComponent.ChildActor` (`self.Tile2`)) :!pure true) (`self.TypeTile_2`))
  (`/Game/Klaft/Blueprint/BP_Tileversoin2.SetupTile` (cast `/Game/Klaft/Blueprint/BP_Tileversoin2` (`ChildActorComponent.ChildActor` (`self.Tile1`)) :!pure true) (`self.TypeTile`)))

(fn `UserConstructionScript`
  (if (`self.TransitionTile?`)
    (set `self.IndexTransition` (+ (`self.RegionIndex`) 1)))
  (`self.ConstructionStr`
    (:`then_3`
      (if (`|EnumEquality` (`self.TypeTile`) "NewEnumerator0")
        (bind _output_get (set `self.TypeTile_2` (select `int` (`KismetMathLibrary.RandomIntegerInRange` 0 2) :`0` "NewEnumerator9" :`1` "NewEnumerator10" :`2` "NewEnumerator5" :!type "/Game/Klaft/EListTypeTile Enum")))
        (if (`|EnumEquality` _output_get "NewEnumerator10")
          (set `self.Enemy_T2` true))))))