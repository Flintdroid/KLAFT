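; Board tile Blueprint whose type (forest, road, mountain, village, boss zones and others) determines its mesh.
; SetupTile stores TypeTile, applies the first mesh from the data table row named after that enum value, then runs per-type defaults.
; Those defaults are stubs: every type passes identical movement and monster flags into an empty settings function.
; Random flip logic is disconnected, and the rotate event, construction script and TypeTile OnRep are empty.
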(event `M_RotateTile`)

(fn `GetDataTableInfoTile`
  (returns (ReturnValue :type "/Game/Klaft/Blueprint/ST_TileInfo Structure"))
  (bind _returnvalue (`|GetDataTableRow` (`self.DataInfo`) (`KismetStringLibrary.Conv_StringToName` (`|GetEnumeratorNameAsString` (`self.TypeTile`))))
    (:`then`
      _)
    (:`RowNotFound`
      _))
  (return _returnvalue))

(fn `OnRep_TypeTile`)

(fn `SettingsDefaultByTypeTile`
  (params (`POssibleToMove?` :type Boolean) (ClassMonter :type "/Game/CoreKlaft/BP_Character Class Reference") (`PossibleMonster?` :type Boolean))
  (`|ExecutionSequence`))

(fn `SetupDefaultSettingsTille`
  (switch `/Game/Klaft/EListTypeTile` (`self.TypeTile`)
    (:`NewEnumerator0`
      (`self.SettingsDefaultByTypeTile` true))
    (:`NewEnumerator1`
      (`self.SettingsDefaultByTypeTile` true))
    (:`NewEnumerator2`
      (`self.SettingsDefaultByTypeTile` true))
    (:`NewEnumerator3`
      (`self.SettingsDefaultByTypeTile` true))
    (:`NewEnumerator4`
      (`self.SettingsDefaultByTypeTile` true))
    (:`NewEnumerator5`
      (`self.SettingsDefaultByTypeTile` true))
    (:`NewEnumerator6`
      (`self.SettingsDefaultByTypeTile` true))
    (:`NewEnumerator7`
      (`self.SettingsDefaultByTypeTile` true))
    (:`NewEnumerator8`
      (`self.SettingsDefaultByTypeTile` true))
    (:`NewEnumerator9`
      (`self.SettingsDefaultByTypeTile` true))
    (:`NewEnumerator10`
      (`self.SettingsDefaultByTypeTile` true))))

(fn `SetupTile`
  (params (TypeTile :type "/Game/Klaft/EListTypeTile Enum" :default "NewEnumerator0"))
  (set `self.TypeTile` TypeTile)
  (`StaticMeshComponent.SetStaticMesh` (`self.StaticMesh`) (`|GetArrayItem` (`.StaticMesh_9_B53066AD44772DD33A8B2BA633DFCB77` (break `/Game/Klaft/Blueprint/ST_TileInfo` (`self.GetDataTableInfoTile`)))))
  (`self.SetupDefaultSettingsTille`))

(fn `UserConstructionScript`)